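; Player HUD Blueprint that relays chat messages and bug-report results to on-screen UI.
; AddMessageBP casts the owning pawn to InvadedPlayer, finds the UIChatWindow state in its state machine and passes the message to that chat window.
; ReportBugComplete opens a brief notification box with the success flag appended to its text.
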(event EventBeginPlay)

(event Collision|EventActorBeginOverlap
  (params (OtherActor :type Actor%20Object%20Reference)))

(event EventTick
  (params (DeltaSeconds :type Float%20%28single-precision%29)))

(event EventAddMessageBP
  (params (Message :type S%20Chat%20Message%20Structure))
  (bind _asinvaded_player (Utilities|Casting|CastToInvadedPlayer (Class|HUD|GetOwningPawn)))
  (bind _asui_chat_window (Utilities|Casting|CastToUI_ChatWindow (Class|InvadedStateMachine|FindStatebyName (Class|InvadedPlayer|GetInvadedStateMachine _asinvaded_player) "UIChatWindow")))
  (Default|AddMessage _asui_chat_window Message))

(event EventReportBugComplete
  (params (bWasSuccessful :type Boolean))
  (Class|PlayerHUD|OpenNotificationBox (Utilities|Text|ToText(String) (Utilities|String|Append (Utilities|String|MakeLiteralString "Bug report was sent") (Utilities|String|ToString(Boolean) bWasSuccessful))) 2.0))

(fn ConstructionScript)