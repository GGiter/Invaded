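; Player controller for Invaded that manages cursor widgets, applies audio volumes and feeds keyboard input to typing battles.
; BeginPlay creates default and hover cursor widgets for swapping via events, then after a delay applies Master, FX and Music volumes through a sound mix.
; In Fight mode, pressed keyboard keys go by display name to the visible UI_TypeBattle found through the pawn's state machine.
; The HUD-actor camera setup is disconnected and never runs.
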(event Custom|ChangeToDefaultMouseIcon
  (Utilities|IsValid (Variables|Default|GetMouseIcon)
    (:Is%20Valid
      (Class|PlayerController|SetMouseCursorWidget "Default" (Variables|Default|GetMouseIcon)))))

(event Custom|ChangeToHoverMouseIcon
  (Utilities|IsValid (Variables|Default|GetHoverIcon)
    (:Is%20Valid
      (Class|PlayerController|SetMouseCursorWidget "Default" (Variables|Default|GetHoverIcon)))))

(event EventEndPlay
  (params (EndPlayReason :type EEndPlayReason%20Enum :default "Destroyed"))
  (CallFunction|ChangetoDefaultMouseIcon))

(event EventPossess
  (params (PossessedPawn :type Pawn%20Object%20Reference)))

(event EventBeginPlay
  (Utilities|FlowControl|Sequence
    (:then_0
      (bind _returnvalue (UserInterface|CreateWidget "/Game/UI/UI_HoverIcon.UI_HoverIcon_C"))
      (Variables|Default|SetHoverIcon _returnvalue))
    (:then_1
      (bind _returnvalue_2 (UserInterface|CreateWidget "/Game/UI/UI_MouseIcon.UI_MouseIcon_C"))
      (Variables|Default|SetMouseIcon _returnvalue_2)
      (Class|PlayerController|SetMouseCursorWidget "Default" _returnvalue_2))
    (:then_2
      (Utilities|FlowControl|Delay 2.0)
      (Audio|SetSoundMixClassOverride "/Game/Audio/MasterMuteMix.MasterMuteMix" "/Game/Audio/SoundFX.SoundFX" (Class|SoundSettings|GetFXVolume) 1.0 1.0 true)
      (Audio|SetSoundMixClassOverride "/Game/Audio/MasterMuteMix.MasterMuteMix" "/Game/Audio/Master.Master" (Class|SoundSettings|GetMasterVolume) 1.0 1.0 true)
      (Audio|SetSoundMixClassOverride "/Game/Audio/MasterMuteMix.MasterMuteMix" "/Game/Audio/Music.Music" (Class|SoundSettings|GetMusicVolume) 1.0 1.0 true))))

(event Input|KeyboardEvents|AnyKey
  (params (Key :type Key%20Structure :default "None"))
  (:Pressed
    (Utilities|FlowControl|Delay 0.01)
    (if (Class|KismetInputLibrary|KeyIsKeyboardKey Key)
      (bind _asinvaded_player (Utilities|Casting|CastToInvadedPlayer (Pawn|GetControlledPawn)))
      (if (Utilities|Enum|Equal(Enum) (Class|InvadedData|GetPlayerMode (Class|InvadedCharacter|GetInvadedPS _asinvaded_player)) "PM_Fight")
        (Utilities|IsValid (Class|InvadedPlayer|GetInvadedStateMachine _asinvaded_player)
          (:Is%20Valid
            (Utilities|IsValid (Class|InvadedStateMachine|FindStatebyName (Class|InvadedPlayer|GetInvadedStateMachine _asinvaded_player) "UIGameWord")
              (:Is%20Valid
                (if (Utilities|Enum|Equal(Enum) (Widget|GetVisibility (Class|InvadedStateMachine|FindStatebyName (Class|InvadedPlayer|GetInvadedStateMachine _asinvaded_player) "UIGameWord")) "Visible")
                  (bind _asui_type_battle (Utilities|Casting|CastToUI_TypeBattle (Class|InvadedStateMachine|FindStatebyName (Class|InvadedPlayer|GetInvadedStateMachine _asinvaded_player) "UIGameWord")))
                  (Default|PressedKey _asui_type_battle (Utilities|String|ToString(Text) (Class|KismetInputLibrary|KeyGetDisplayName Key))))))))))))

(fn ConstructionScript)