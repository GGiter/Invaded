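; Spectator player Blueprint with a HUD on a Screen widget component and a toggleable Hand component.
; On BeginPlay, after a short delay, it hands its state machine to the UI_NewHUD widget, triggers its enter event and caches it.
; ToggleHUD shows the Hand and plays the EnableUI sequence, or reverses it and hides the Hand after a fixed delay.
; CollapseHUD always runs the closing path.
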(event EventBeginPlay
  (Utilities|FlowControl|Delay 1.0)
  (bind _asui_new_hud (Utilities|Casting|CastToUI_NewHUD (UserInterface|GetUserWidgetObject (Variables|Default|GetScreen))))
  (Variables|/Script/Invaded.InvadedMenuState|SetStateMachine _asui_new_hud (Class|SpectatorPlayer|GetStateMachine))
  (Class|InvadedMenuState|ReceiveonEnter _asui_new_hud)
  (Variables|Default|SetMainGameWidget _asui_new_hud))

(event EventToggleHUD
  (if (Variables|Default|GetEnabled)
    (Variables|Default|SetEnabled false)
    (Class|MovieSceneSequencePlayer|PlayReverse (Variables|/Script/ActorSequence.ActorSequenceComponent|GetSequencePlayer (Variables|Default|GetEnableUI)))
    (Utilities|FlowControl|Delay 1.4)
    (Rendering|SetVisibility (Variables|Default|GetHand) false true)
    (else
      (Variables|Default|SetEnabled true)
      (Rendering|SetVisibility (Variables|Default|GetHand) true true)
      (Sequencer|Player|Play (Variables|/Script/ActorSequence.ActorSequenceComponent|GetSequencePlayer (Variables|Default|GetEnableUI)) :!class /Script/MovieScene.MovieSceneSequencePlayer))))

(event EventCollapseHUD
  (Variables|Default|SetEnabled false)
  (Class|MovieSceneSequencePlayer|PlayReverse (Variables|/Script/ActorSequence.ActorSequenceComponent|GetSequencePlayer (Variables|Default|GetEnableUI)))
  (Utilities|FlowControl|Delay 1.4)
  (Rendering|SetVisibility (Variables|Default|GetHand) false true))

(fn ConstructionScript)