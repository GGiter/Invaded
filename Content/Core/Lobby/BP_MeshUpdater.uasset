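; Lobby preview actor that shows the player's character mesh, socketed weapon and flag for customization.
; Possess applies saved MenuPS indices and LobbyPS colors, while a timeline blends the first CameraActor's camera to CameraPoint; UnPossess reverses it, pushing the widget's Customization or Lobby state on finish.
; Next/Previous events cycle wrapping mesh, weapon and flag arrays without writing selections back.
; Flag textures and colors go through a dynamic material instance, recreated on each texture change.
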(event Custom|Possess
  (params (Widget :type Invaded%20State%20Machine%20Object%20Reference))
  (bind _returnvalue (Widget|GetOwningPlayer Widget))
  (bind _flagmaterialdyn (Variables|Default|GetFlagMaterialDyn))
  (bind _playerstate (Variables|/Script/Engine.Controller|GetPlayerState _returnvalue))
  (Utilities|FlowControl|Sequence
    (:then_0
      (bind _asmenu_ps (Utilities|Casting|CastToMenuPS _playerstate))
      (Variables|Default|SetWeaponIndex (Class|MenuPS|GetWeaponIndex _asmenu_ps))
      (Variables|Default|SetMeshIndex (Class|MenuPS|GetMeshIndex _asmenu_ps))
      (Variables|Default|SetFlagIndex (Class|MenuPS|GetFlagTextureIndex _asmenu_ps)))
    (:then_1
      (Components|StaticMesh|SetStaticMesh (Variables|Default|GetStaticMesh) (Utilities|Array|Get(acopy) (Variables|Default|GetWeaponArray) (Variables|Default|GetWeaponIndex))))
    (:then_2
      (Class|SkinnedMeshComponent|SetSkeletalMesh (Variables|Default|GetSkeletalMesh) (Utilities|Array|Get(acopy) (Variables|Default|GetMeshArray) (Variables|Default|GetMeshIndex)) true)
      (CallFunction|PlayAnimation))
    (:then_3
      (bind _outactors (Actor|GetAllActorsOfClass "/Script/Engine.CameraActor"))
      (bind _output_get (Variables|Default|SetStartLocation (Transformation|GetWorldTransform (Variables|/Script/Engine.CameraActor|GetCameraComponent (Utilities|Array|Get(acopy) _outactors)))))
      (bind (_direction _newtrack_0) (Timeline|Timeline_0 PlayFromStart)
        (:Update
          (Transformation|SetWorldTransform (Variables|/Script/Engine.CameraActor|GetCameraComponent (Utilities|Array|Get(acopy) _outactors)) (Math|Transform|Lerp(Transform) _output_get (Transformation|GetWorldTransform (Variables|Default|GetCameraPoint)) _newtrack_0) false false))
        (:Finished
          (switch Utilities|FlowControl|Switch|SwitchonETimelineDirection _direction
            (:Forward
              (Class|InvadedStateMachine|PushState Widget "Customization"))
            (:Backward
              (Class|InvadedStateMachine|PushState (stale Custom|UnPossess Widget) "Lobby"))))))
    (:then_4
      (CallFunction|UpdateFlagTexture (Variables|Default|GetFlagIndex)))
    (:then_5
      (Utilities|IsValid _flagmaterialdyn
        (:Is%20Valid
          (bind _aslobby_ps (Utilities|Casting|CastToLobbyPS _playerstate))
          (Rendering|Material|SetVectorParameterValue _flagmaterialdyn "P_Color1" (Class|MenuPS|GetPlayerColor _aslobby_ps) :!class /Script/Engine.MaterialInstanceDynamic)
          (Rendering|Material|SetVectorParameterValue _flagmaterialdyn "P_Color2" (Class|MenuPS|GetFlagColor _aslobby_ps) :!class /Script/Engine.MaterialInstanceDynamic))))))

(event Custom|UnPossess
  (params (Widget :type Invaded%20State%20Machine%20Object%20Reference))
  (bind (_direction _newtrack_0) (Timeline|Timeline_0 ReverseFromEnd)
    (:Update
      (Transformation|SetWorldTransform (Variables|/Script/Engine.CameraActor|GetCameraComponent (Utilities|Array|Get(acopy) (stale Custom|Possess _outactors))) (Math|Transform|Lerp(Transform) (stale Custom|Possess _output_get) (Transformation|GetWorldTransform (Variables|Default|GetCameraPoint)) _newtrack_0) false false))
    (:Finished
      (switch Utilities|FlowControl|Switch|SwitchonETimelineDirection _direction
        (:Forward
          (Class|InvadedStateMachine|PushState (stale Custom|Possess Widget) "Customization"))
        (:Backward
          (Class|InvadedStateMachine|PushState Widget "Lobby"))))))

(event Custom|UpdateColor
  (params (P_Color1 :type Linear%20Color%20Structure) (P_Color2 :type Linear%20Color%20Structure))
  (bind _flagmaterialdyn (Variables|Default|GetFlagMaterialDyn))
  (Utilities|IsValid (Variables|Default|GetPlayerController)
    (:Is%20Valid
      (Utilities|IsValid _flagmaterialdyn
        (:Is%20Valid
          (Rendering|Material|SetVectorParameterValue _flagmaterialdyn "P_Color1" P_Color1 :!class /Script/Engine.MaterialInstanceDynamic)
          (Rendering|Material|SetVectorParameterValue _flagmaterialdyn "P_Color2" P_Color2 :!class /Script/Engine.MaterialInstanceDynamic))))))

(event Custom|NextWeapon
  (bind _weaponarray (Variables|Default|GetWeaponArray))
  (bind _returnvalue (Utilities|Array|Length _weaponarray))
  (bind _returnvalue_2 (- _returnvalue 1))
  (if (> (+ (Variables|Default|GetWeaponIndex) 1) _returnvalue_2)
    (Variables|Default|SetWeaponIndex 0)
    (else
      (bind _output_get (Variables|Default|SetWeaponIndex (Math|Integer|Clamp(Integer) (+ (Variables|Default|GetWeaponIndex) 1) 0 _returnvalue_2)))))
  (Components|StaticMesh|SetStaticMesh (Variables|Default|GetStaticMesh) (Utilities|Array|Get(acopy) (Variables|Default|GetWeaponArray) _output_get)))

(event Custom|PreviousWeapon
  (bind _weaponarray (Variables|Default|GetWeaponArray))
  (bind _returnvalue (Utilities|Array|Length _weaponarray))
  (bind _returnvalue_2 (- _returnvalue 1))
  (if (< (+ (Variables|Default|GetWeaponIndex) -1) 0)
    (Variables|Default|SetWeaponIndex _returnvalue_2)
    (else
      (Variables|Default|SetWeaponIndex (Math|Integer|Clamp(Integer) (+ (Variables|Default|GetWeaponIndex) -1) 0 _returnvalue_2))))
  (Components|StaticMesh|SetStaticMesh (Variables|Default|GetStaticMesh) (Utilities|Array|Get(acopy) (Variables|Default|GetWeaponArray) (Math|Integer|Clamp(Integer) (+ (Variables|Default|GetWeaponIndex) -1) 0 _returnvalue_2))))

(event Custom|NextPlayerMesh
  (bind _mesharray (Variables|Default|GetMeshArray))
  (bind _returnvalue (Utilities|Array|Length _mesharray))
  (bind _returnvalue_2 (- _returnvalue 1))
  (if (> (+ (Variables|Default|GetMeshIndex) 1) _returnvalue_2)
    (Variables|Default|SetMeshIndex 0)
    (else
      (bind _output_get (Variables|Default|SetMeshIndex (Math|Integer|Clamp(Integer) (+ (Variables|Default|GetMeshIndex) 1) 0 _returnvalue_2)))))
  (Class|SkinnedMeshComponent|SetSkeletalMesh (Variables|Default|GetSkeletalMesh) (Utilities|Array|Get(acopy) (Variables|Default|GetMeshArray) _output_get) true)
  (CallFunction|PlayAnimation)
  (for (_array_element _array_index) (Variables|/Script/Engine.SkeletalMesh|GetMaterials (Utilities|Array|Get(acopy) (Variables|Default|GetMeshArray) _output_get))
    (Rendering|Material|SetMaterial (Variables|Default|GetSkeletalMesh) _array_index (.materialinterface _array_element))))

(event Custom|PreviousPlayerMesh
  (bind _mesharray (Variables|Default|GetMeshArray))
  (bind _returnvalue (Utilities|Array|Length _mesharray))
  (bind _returnvalue_2 (- _returnvalue 1))
  (if (< (+ (Variables|Default|GetMeshIndex) -1) 0)
    (Variables|Default|SetMeshIndex _returnvalue_2)
    (else
      (bind _output_get (Variables|Default|SetMeshIndex (Math|Integer|Clamp(Integer) (+ (Variables|Default|GetMeshIndex) -1) 0 _returnvalue_2)))))
  (Class|SkinnedMeshComponent|SetSkeletalMesh (Variables|Default|GetSkeletalMesh) (Utilities|Array|Get(acopy) (Variables|Default|GetMeshArray) _output_get) true)
  (CallFunction|PlayAnimation)
  (for (_array_element _array_index) (Variables|/Script/Engine.SkeletalMesh|GetMaterials (Utilities|Array|Get(acopy) (Variables|Default|GetMeshArray) _output_get))
    (Rendering|Material|SetMaterial (Variables|Default|GetSkeletalMesh) _array_index (.materialinterface _array_element))))

(event Custom|PlayAnimation
  (switch int (Variables|Default|GetMeshIndex)
    (:0
      (Components|Animation|PlayAnimation (Variables|Default|GetSkeletalMesh) "/Game/Anims/StandardSkeleton/Anims/Rifle_Idle.Rifle_Idle" true))
    (:1
      (Components|Animation|PlayAnimation (Variables|Default|GetSkeletalMesh) "/Game/Anims/StandardSkeleton/Anims/Rifle_Idle.Rifle_Idle" true :!label _label))
    (:2
      (goto _label))))

(event Custom|NextFlagTexture
  (bind _flagtexturesarray (Variables|Default|GetFlagTexturesArray))
  (bind _returnvalue (Utilities|Array|Length _flagtexturesarray))
  (bind _returnvalue_2 (- _returnvalue 1))
  (if (> (+ (Variables|Default|GetFlagIndex) 1) _returnvalue_2)
    (Variables|Default|SetFlagIndex 0)
    (else
      (bind _output_get (Variables|Default|SetFlagIndex (Math|Integer|Clamp(Integer) (+ (Variables|Default|GetFlagIndex) 1) 0 _returnvalue_2)))))
  (CallFunction|UpdateFlagTexture _output_get))

(event Custom|PreviousFlagTexture
  (bind _flagtexturesarray (Variables|Default|GetFlagTexturesArray))
  (bind _returnvalue (Utilities|Array|Length _flagtexturesarray))
  (bind _returnvalue_2 (- _returnvalue 1))
  (if (< (+ (Variables|Default|GetFlagIndex) -1) 0)
    (Variables|Default|SetFlagIndex _returnvalue_2)
    (else
      (bind _output_get (Variables|Default|SetFlagIndex (Math|Integer|Clamp(Integer) (+ (Variables|Default|GetFlagIndex) -1) 0 _returnvalue_2)))))
  (CallFunction|UpdateFlagTexture _output_get))

(event Custom|UpdateFlagTexture
  (params (Index :type Integer))
  (bind _playercontroller (Variables|Default|GetPlayerController))
  (Utilities|FlowControl|Sequence
    (:then_0
      (bind _returnvalue (Rendering|Material|CreateDynamicMaterialInstance (Variables|Default|GetFlagMesh) 0 "/Game/Materials/Flags/M_Flag_Inst.M_Flag_Inst" "None" :!class /Script/Engine.PrimitiveComponent))
      (Rendering|Material|SetTextureParameterValue _returnvalue "ML_Mask" (Utilities|Array|Get(acopy) (Variables|Default|GetFlagTexturesArray) Index))
      (Rendering|Material|SetTextureParameterValue _returnvalue "Symbol" (Utilities|Array|Get(acopy) (Variables|Default|GetFlagTexturesArray2) Index))
      (Rendering|Material|SetTextureParameterValue _returnvalue "AlphaMask" (Utilities|Array|Get(acopy) (Variables|Default|GetFlagTexturesArray) Index))
      (bind _output_get (Variables|Default|SetFlagMaterialDyn _returnvalue))
      (Utilities|IsValid _playercontroller
        (:Is%20Valid
          (bind _aslobby_ps (Utilities|Casting|CastToLobbyPS (Variables|/Script/Engine.Controller|GetPlayerState _playercontroller)))
          (Rendering|Material|SetVectorParameterValue _output_get "P_Color1" (Class|MenuPS|GetPlayerColor _aslobby_ps) :!class /Script/Engine.MaterialInstanceDynamic)
          (Rendering|Material|SetVectorParameterValue _output_get "P_Color2" (Class|MenuPS|GetFlagColor _aslobby_ps) :!class /Script/Engine.MaterialInstanceDynamic))))
    (:then_1
      (Rendering|Material|SetMaterial (Variables|Default|GetFlagMesh) 0 _returnvalue))))

(event EventBeginPlay)

(fn ConstructionScript
  (Transformation|AttachComponentToComponent (Variables|Default|GetStaticMesh) (Variables|Default|GetSkeletalMesh) "WeaponSocket" "KeepRelative" "KeepRelative" "KeepRelative" true))