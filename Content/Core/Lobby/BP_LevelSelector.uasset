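; Lobby actor for picking a level and a grid type, shown as preview meshes and generated grid previews with UI widget updates.
; Next and Previous cycle three level meshes, dissolving them through dynamic material timelines and moving a Niagara effect to the shown mesh.
; Timelines blend the first CameraActor's camera between lobby, level and grid views.
; A spawned BP_GridGenerationCauser finds grid types on the server and builds a scaled-down preview.
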(event Custom|Next
  (params (Widget :type UI%20Level%20Selection%20Object%20Reference))
  (bind _output_get (Variables|Default|SetPreviousIndex (Variables|Default|GetCurrentIndex)))
  (Utilities|FlowControl|Sequence
    (:then_0
      (if (== (+ (Variables|Default|GetCurrentIndex) 1) (Utilities|Array|Length (Variables|Default|GetMeshArray)))
        (Variables|Default|SetCurrentIndex 0)
        (else
          (Variables|Default|SetCurrentIndex (+ (Variables|Default|GetCurrentIndex) 1)))))
    (:then_1
      (CallFunction|ShowNextMesh (Utilities|Array|Get(acopy) (Variables|Default|GetMeshArray) _output_get) (Utilities|Array|Get(acopy) (Variables|Default|GetMeshArray) (Variables|Default|GetCurrentIndex))))
    (:then_2
      (CallFunction|UpdateCurrentLevel Widget))))

(event Custom|Previous
  (params (Widget :type UI%20Level%20Selection%20Object%20Reference))
  (bind _output_get (Variables|Default|SetPreviousIndex (Variables|Default|GetCurrentIndex)))
  (Utilities|FlowControl|Sequence
    (:then_0
      (if (== (+ (Variables|Default|GetCurrentIndex) -1) -1)
        (Variables|Default|SetCurrentIndex (+ (Utilities|Array|Length (Variables|Default|GetMeshArray)) -1))
        (else
          (Variables|Default|SetCurrentIndex (+ (Variables|Default|GetCurrentIndex) -1)))))
    (:then_1
      (CallFunction|ShowNextMesh (Utilities|Array|Get(acopy) (Variables|Default|GetMeshArray) _output_get) (Utilities|Array|Get(acopy) (Variables|Default|GetMeshArray) (Variables|Default|GetCurrentIndex))))
    (:then_2
      (CallFunction|UpdateCurrentLevel Widget))))

(event Custom|PreviousGridType
  (params (Widget :type UI%20Level%20Selection%20Object%20Reference))
  (bind _gridtypesarray (Variables|Default|GetGridTypesArray))
  (bind _returnvalue (Utilities|Array|Length _gridtypesarray))
  (bind _returnvalue_2 (+ _returnvalue -1))
  (if (< (+ (Variables|Default|GetCurrentGridTypeIndex) -1) 0)
    (Variables|Default|SetCurrentGridTypeIndex _returnvalue_2)
    (else
      (Variables|Default|SetCurrentGridTypeIndex (Math|Integer|Clamp(Integer) (+ (Variables|Default|GetCurrentGridTypeIndex) -1) 0 _returnvalue_2))))
  (Class|GridGeneratorFunctionLibrary|DestroyCells (Variables|Default|GetGridGenerator))
  (CallFunction|GenerateGrid)
  (Variables|/Game/UI/Lobby/UI_LevelSelection.UI_LevelSelection_C|SetGridName Widget (Utilities|Array|Get(acopy) (Variables|Default|GetGridTypesArray) (Variables|Default|GetCurrentGridTypeIndex))))

(event Custom|GenerateGrid
  (Class|GridGeneratorFunctionLibrary|GenerateBuildData (Variables|Default|GetGridGenerator) (Utilities|Struct|MakeGridGeneratorInfo "0.000000,0.000000,0.000000" (Utilities|Array|MakeArray "") (Utilities|Array|MakeArray "CT_None") (Transformation|GetWorldLocation (Variables|Default|GetGridLocaion)) "0.000000,0.000000,0.000000" 1e+01 (Utilities|Array|Get(acopy) (Variables|Default|GetGridTypesArray) (Variables|Default|GetCurrentGridTypeIndex))) 0.1))

(event Custom|ShowMesh
  (params (StaticMeshComponent :type Static%20Mesh%20Component%20Object%20Reference))
  (Transformation|SetWorldTransform (Variables|Default|GetNiagara) (Transformation|GetWorldTransform StaticMeshComponent) false false)
  (bind _newtrack_0 (Timeline|Timeline_0 ReverseFromEnd)
    (:Update
      (bind _asmaterial_instance_dynamic (Utilities|Casting|CastToMaterialInstanceDynamic (Rendering|Material|GetMaterial StaticMeshComponent 0)))
      (Rendering|Material|SetScalarParameterValue _asmaterial_instance_dynamic "DissolveAmount" _newtrack_0 :!class /Script/Engine.MaterialInstanceDynamic)
      (for _index (range 0 (Utilities|Array|Length (Rendering|Material|GetMaterials StaticMeshComponent)))
        (Rendering|Material|SetMaterial StaticMeshComponent _index _asmaterial_instance_dynamic)))))

(event Custom|ShowNextMesh
  (params (PreviousStaicMeshComponent :type Static%20Mesh%20Component%20Object%20Reference) (NextStaticMeshComponent :type Static%20Mesh%20Component%20Object%20Reference))
  (Utilities|FlowControl|Sequence
    (:then_0
      (for _array_element (Variables|Default|GetMeshArray)
        (if (or (== _array_element PreviousStaicMeshComponent) (== _array_element NextStaticMeshComponent))
          (bind _asmaterial_instance_dynamic (Utilities|Casting|CastToMaterialInstanceDynamic (Rendering|Material|GetMaterial _array_element 0)))
          (Rendering|Material|SetScalarParameterValue _asmaterial_instance_dynamic "DissolveAmount" 1.0 :!class /Script/Engine.MaterialInstanceDynamic)
          (for _index (range 0 (Utilities|Array|Length (Rendering|Material|GetMaterials _array_element)))
            (Rendering|Material|SetMaterial _array_element _index _asmaterial_instance_dynamic)))))
    (:then_1
      (bind _newtrack_0 (Timeline|Timeline_2 Play)
        (:Update
          (bind _asmaterial_instance_dynamic_2 (Utilities|Casting|CastToMaterialInstanceDynamic (Rendering|Material|GetMaterial PreviousStaicMeshComponent 0)))
          (Rendering|Material|SetScalarParameterValue _asmaterial_instance_dynamic_2 "DissolveAmount" _newtrack_0 :!class /Script/Engine.MaterialInstanceDynamic)
          (for _index_2 (range 0 (Utilities|Array|Length (Rendering|Material|GetMaterials PreviousStaicMeshComponent)))
            (Rendering|Material|SetMaterial PreviousStaicMeshComponent _index_2 _asmaterial_instance_dynamic_2)))
        (:Finished
          (CallFunction|ShowMesh NextStaticMeshComponent))))))

(event Custom|Possess
  (params (Widget :type UI%20Level%20Selection%20Object%20Reference))
  (Utilities|FlowControl|Sequence
    (:then_0
      (bind _outactors (Actor|GetAllActorsOfClass "/Script/Engine.CameraActor"))
      (Variables|Default|SetPlayerCamera (Variables|/Script/Engine.CameraActor|GetCameraComponent (Utilities|Array|Get(acopy) _outactors)))
      (bind _output_get (Variables|Default|SetStartLocation (Transformation|GetWorldTransform (Variables|/Script/Engine.CameraActor|GetCameraComponent (Utilities|Array|Get(acopy) _outactors)))))
      (bind (_direction _newtrack_0) (Timeline|Timeline_1 PlayFromStart)
        (:Update
          (Transformation|SetWorldTransform (Variables|/Script/Engine.CameraActor|GetCameraComponent (Utilities|Array|Get(acopy) _outactors)) (Math|Transform|Lerp(Transform) _output_get (Transformation|GetWorldTransform (Variables|Default|GetCameraPoint)) _newtrack_0 "EulerInterp") false false))
        (:Finished
          (switch Utilities|FlowControl|Switch|SwitchonETimelineDirection _direction
            (:Forward
              (Class|InvadedStateMachine|PushState (Variables|/Script/Invaded.InvadedMenuState|GetStateMachine Widget) "LevelSelection"))
            (:Backward
              (Class|InvadedStateMachine|PushState (stale Custom|UnPossess Widget) "Lobby"))))))
    (:then_1
      (CallFunction|UpdateCurrentLevel Widget))))

(event Custom|UnPossess
  (params (Widget :type Invaded%20State%20Machine%20Object%20Reference))
  (bind (_direction _newtrack_0) (Timeline|Timeline_1 ReverseFromEnd)
    (:Update
      (Transformation|SetWorldTransform (Variables|/Script/Engine.CameraActor|GetCameraComponent (Utilities|Array|Get(acopy) (stale Custom|Possess _outactors))) (Math|Transform|Lerp(Transform) (stale Custom|Possess _output_get) (Transformation|GetWorldTransform (Variables|Default|GetCameraPoint)) _newtrack_0 "EulerInterp") false false))
    (:Finished
      (switch Utilities|FlowControl|Switch|SwitchonETimelineDirection _direction
        (:Forward
          (Class|InvadedStateMachine|PushState (Variables|/Script/Invaded.InvadedMenuState|GetStateMachine (stale Custom|Possess Widget)) "LevelSelection"))
        (:Backward
          (Class|InvadedStateMachine|PushState Widget "Lobby"))))))

(event Custom|GoToGridSelection
  (params (Widget :type User%20Widget%20Object%20Reference))
  (Utilities|FlowControl|Sequence
    (:then_0
      (bind _outactors (Actor|GetAllActorsOfClass "/Script/Engine.CameraActor"))
      (bind _output_get (Variables|Default|SetStartLocationGrid (Transformation|GetWorldTransform (Variables|/Script/Engine.CameraActor|GetCameraComponent (Utilities|Array|Get(acopy) _outactors)))))
      (bind _newtrack_0 (Timeline|Timeline_3 PlayFromStart)
        (:Update
          (Transformation|SetWorldTransform (Variables|/Script/Engine.CameraActor|GetCameraComponent (Utilities|Array|Get(acopy) _outactors)) (Math|Transform|Lerp(Transform) _output_get (Transformation|GetWorldTransform (Variables|Default|GetGirdCameraPoint)) _newtrack_0) false false))))
    (:then_1
      (Widget|SetVisibility Widget "Visible")
      (CallFunction|GenerateGrid)
      (for _array_element (Variables|Default|GetMeshArray)
        (Development|SetHiddeninGame _array_element true false)))))

(event Custom|UpdateCurrentLevel
  (params (Widget :type UI%20Level%20Selection%20Object%20Reference))
  (Variables|/Game/UI/Lobby/UI_LevelSelection.UI_LevelSelection_C|SetLevelName Widget (Utilities|Array|Get(acopy) (Variables|Default|GetDisplayNameArray) (Variables|Default|GetCurrentIndex))))

(event Custom|GoToLevelSelection
  (params (Widget :type User%20Widget%20Object%20Reference))
  (Utilities|FlowControl|Sequence
    (:then_0
      (bind _newtrack_0 (Timeline|Timeline_3 ReverseFromEnd)
        (:Update
          (Transformation|SetWorldTransform (Variables|/Script/Engine.CameraActor|GetCameraComponent (Utilities|Array|Get(acopy) (stale Custom|GoToGridSelection _outactors))) (Math|Transform|Lerp(Transform) (stale Custom|GoToGridSelection _output_get) (Transformation|GetWorldTransform (Variables|Default|GetGirdCameraPoint)) _newtrack_0) false false))))
    (:then_1
      (Widget|SetVisibility Widget "Visible")
      (Class|GridGeneratorFunctionLibrary|DestroyCells (Variables|Default|GetGridGenerator))
      (for _array_element (Variables|Default|GetMeshArray)
        (Development|SetHiddeninGame _array_element false false)))))

(event Custom|NextGridType
  (params (Widget :type UI%20Level%20Selection%20Object%20Reference))
  (bind _gridtypesarray (Variables|Default|GetGridTypesArray))
  (bind _returnvalue (Utilities|Array|Length _gridtypesarray))
  (bind _returnvalue_2 (+ _returnvalue -1))
  (if (> (+ (Variables|Default|GetCurrentGridTypeIndex) 1) _returnvalue_2)
    (Variables|Default|SetCurrentGridTypeIndex 0)
    (else
      (Variables|Default|SetCurrentGridTypeIndex (Math|Integer|Clamp(Integer) (+ (Variables|Default|GetCurrentGridTypeIndex) 1) 0 _returnvalue_2))))
  (Class|GridGeneratorFunctionLibrary|DestroyCells (Variables|Default|GetGridGenerator))
  (CallFunction|GenerateGrid)
  (Variables|/Game/UI/Lobby/UI_LevelSelection.UI_LevelSelection_C|SetGridName Widget (Utilities|Array|Get(acopy) (Variables|Default|GetGridTypesArray) (Variables|Default|GetCurrentGridTypeIndex))))

(event Collision|EventActorBeginOverlap
  (params (OtherActor :type Actor%20Object%20Reference)))

(event EventTick
  (params (DeltaSeconds :type Float%20%28single-precision%29)))

(event EventBeginPlay
  (Utilities|FlowControl|Sequence
    (:then_0
      (CallFunction|ShowMesh (Variables|Default|GetLevel2))
      (bind _returnvalue (Game|SpawnActorfromClass "/Game/Core/Lobby/BP_GridGenerationCauser.BP_GridGenerationCauser_C" (Math|Transform|MakeTransform "0, 0, 0") "Undefined" 0 0))
      (Variables|Default|SetGridGenerator _returnvalue))
    (:then_1
      (if (Networking|IsServer)
        (Variables|Default|SetGridTypesArray (Class|GridGeneratorFunctionLibrary|FindMaps (Variables|Default|GetGridGenerator)))))))

(fn ConstructionScript
  (Utilities|FlowControl|Sequence
    (:then_0
      (bind _output_get (Variables|Default|SetMeshArray (Utilities|Array|MakeArray (Variables|Default|GetLevel2) (Variables|Default|GetLevel3) (Variables|Default|GetLevel4))))
      (for _array_element _output_get
        (bind _returnvalue (Rendering|Material|CreateDynamicMaterialInstance _array_element 0 "/Game/Core/Lobby/M_Highlight_Inst.M_Highlight_Inst" "None" :!class /Script/Engine.PrimitiveComponent))
        (for _index (range 0 2)
          (Rendering|Material|SetMaterial _array_element 0 _returnvalue))
        (Utilities|Array|Add (Variables|Default|GetMaterialArray) _returnvalue)))))

(fn GetCurrentMapInfo
  (return (Utilities|Array|Get(acopy) (Variables|Default|GetMapArray) (Variables|Default|GetCurrentIndex))))