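; Game Instance for Invaded that hosts and joins multiplayer sessions and launches singleplayer games.
; Hosting maps ports, creates an Advanced Session carrying name and password properties, then opens a listen-server level; singleplayer skips both mapping and session.
; Joining compares the password client-side, proceeding if none is found.
; Init and Shutdown manage port mapping, while Steam invites and network errors spawn UI widgets.
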(event Custom|HostSession
  (params (Password :type String) (IsLan :type Boolean))
  (Class|InvadedGI|AddPortMapping 7777)
  (Class|InvadedGI|AddPortMapping 27015)
  (|AdvancedSession (Utilities|Array|MakeArray (Class|AdvancedSessionsLibrary|MakeLiteralSessionPropertyString "GAMENAME" "QUICKGAME") (Class|AdvancedSessionsLibrary|MakeLiteralSessionPropertyString "CPASSWORD" Password)) (Game|GetPlayerController 0) 4 0 false true false true true false true true true
    (:OnSuccess
      (Game|OpenLevel(byName) "LobbyLevel" false "listen"))
    (:OnFailure
      (Development|PrintString "Failure"))))

(event Custom|JoinSession
  (params (Session :type Blueprint%20Session%20Result%20Structure) (Password :type String))
  (Development|PrintString "Joining")
  (bind _output_get (Variables|Default|SetSessionRef Session))
  (bind _extrasettings (Class|AdvancedSessionsLibrary|GetExtraSettings _output_get))
  (bind _settingvalue (Class|AdvancedSessionsLibrary|GetSessionPropertyString _extrasettings "CPASSWORD")
    (:Found
      (if (Utilities|Enum|Equal(Enum) _settingvalue Password)
        (|JoinSession (Game|GetPlayerController 0) Session :!label _label)
        (else
          (Development|PrintString "WrongPassword"))))
    (:NotFound
      (goto _label))
    (:WrongType
      (goto _label))))

(event Custom|HostSessionWithParameters
  (params (IsLan :type Boolean) (GameName :type String) (MapName :type String) (Password :type String) (Singleplayer :type Boolean))
  (bind _returnvalue (Utilities|String|StringToName MapName))
  (if Singleplayer
    (Game|OpenLevel(byName) (Utilities|String|StringToName MapName) true "?listen?singleplayer=true")
    (else
      (Class|InvadedGI|AddPortMapping 7777)
      (Class|InvadedGI|AddPortMapping 27015)
      (|AdvancedSession (Utilities|Array|MakeArray (Class|AdvancedSessionsLibrary|MakeLiteralSessionPropertyString "GAMENAME" GameName) (Class|AdvancedSessionsLibrary|MakeLiteralSessionPropertyString "CPASSWORD" Password) (Class|AdvancedSessionsLibrary|MakeLiteralSessionPropertyBool "SINGLEPLAYER" Singleplayer)) (Game|GetPlayerController 0) 4 0 IsLan true false true true false true true true
        (:OnSuccess
          (if Singleplayer
            (Game|OpenLevel(byName) _returnvalue true "?listen?singleplayer=true")
            (else
              (Game|OpenLevel(byName) _returnvalue true "listen"))))
        (:OnFailure
          (Development|PrintString "Failure"))))))

(event EventShutdown
  (Class|InvadedGI|RemovePortMapping 7777)
  (Class|InvadedGI|RemovePortMapping 27015))

(event EventInit
  (Class|InvadedGI|InitPortMapping))

(event EventOnSessionInviteAccepted
  (params (LocalPlayerNum :type Integer) (PersonInvited :type BP%20Unique%20Net%20Id%20Structure) (SessionToJoin :type Blueprint%20Session%20Result%20Structure%20%28by%20ref%29))
  (bind _returnvalue (UserInterface|CreateWidget "/Game/UI/Lobby/UI_SteamInvite.UI_SteamInvite_C" (Game|GetPlayerController 0) PersonInvited SessionToJoin))
  (UserInterface|Viewport|AddtoViewport _returnvalue 0))

(event EventHandleNetworkError
  (params (FailureType :type ENetworkFailure%20Enum :default "NetDriverAlreadyExists") (bIsServer :type Boolean))
  (bind _returnvalue (UserInterface|CreateWidget "/Game/UI/UI_NetworkError.UI_NetworkError_C" 0 FailureType))
  (UserInterface|Viewport|AddtoViewport _returnvalue 0))