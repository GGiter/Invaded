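; BP_LobbyGM is the lobby game mode, which strips multiplayer-only content from the level when the game runs standalone.
; After a short delay on BeginPlay, it sets IsSinglePlayer, then hides static mesh and text render actors tagged "Multiplayer".
; It also scans every actor in the level and destroys any component carrying that tag.
; Tick and OnLogout are empty.
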(event EventBeginPlay
  (Utilities|FlowControl|Delay 0.2)
  (if (Class|KismetSystemLibrary|IsStandalone)
    (Variables|Default|SetIsSinglePlayer true)
    (Utilities|FlowControl|Sequence
      (:then_0
        (bind _outactors (Actor|GetAllActorswithTag "Multiplayer"))
        (for _array_element _outactors
          (bind _asstatic_mesh_actor (Utilities|Casting|CastToStaticMeshActor _array_element)
            (:then
              (Rendering|SetVisibility (Variables|/Script/Engine.StaticMeshActor|GetStaticMeshComponent _asstatic_mesh_actor) false true))
            (:CastFailed
              (bind _astext_render_actor (Utilities|Casting|CastToTextRenderActor _array_element))
              (Rendering|SetVisibility (Variables|/Script/Engine.TextRenderActor|GetTextRender _astext_render_actor) false true)))))
      (:then_1
        (bind _outactors_2 (Actor|GetAllActorsOfClass "/Script/Engine.Actor"))
        (for _array_element_2 _outactors_2
          (for _array_element_3 (Actor|GetComponentsbyTag _array_element_2 "/Script/Engine.ActorComponent" "Multiplayer")
            (Components|DestroyComponent _array_element_3)))))))

(event EventTick
  (params (DeltaSeconds :type Float%20%28single-precision%29)))

(event EventOnLogout
  (params (ExitingController :type Controller%20Object%20Reference)))

(fn ConstructionScript)